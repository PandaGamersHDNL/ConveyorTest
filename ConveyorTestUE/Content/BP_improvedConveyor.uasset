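; Spline-based conveyor actor that switches the player pawn into and out of conveyor movement.
; The construction script adds trigger boxes at the start and end of the spline.
; Entering the start box passes the spline to PlayerPawn_BP, enables its conveyor move and resets its travel distance; entering the end box disables the move.
; Movement along the spline is left to the pawn.
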(event `self.BeginBox.OnComponentBeginOverlap`
  (params (OverlappedComponent :type "PrimitiveComponent Object Reference") (OtherActor :type "Actor Object Reference") (OtherComp :type "PrimitiveComponent Object Reference") (OtherBodyIndex :type Integer) (bFromSweep :type Boolean) (SweepResult :type "HitResult Structure (by ref)"))
  (bind _asplayer_pawn_bp (cast `/Game/PlayerPawn_BP` OtherActor)
    (:`then`
      (`/Game/PlayerPawn_BP.SetMove` _asplayer_pawn_bp true (`self.Spline`))
      (set `/Game/PlayerPawn_BP.ConveyorDistance` 0.0 _asplayer_pawn_bp))
    (:`CastFailed`
      (`KismetSystemLibrary.PrintString` "fail"))))

(event `self.EndBox.OnComponentBeginOverlap`
  (params (OverlappedComponent :type "PrimitiveComponent Object Reference") (OtherActor :type "Actor Object Reference") (OtherComp :type "PrimitiveComponent Object Reference") (OtherBodyIndex :type Integer) (bFromSweep :type Boolean) (SweepResult :type "HitResult Structure (by ref)"))
  (bind _asplayer_pawn_bp (cast `/Game/PlayerPawn_BP` OtherActor))
  (`/Game/PlayerPawn_BP.SetMove` _asplayer_pawn_bp false (`self.Spline`)))

(fn `UserConstructionScript`
  (locals (NewLocalVar_0 :type "BoxComponent Object Reference"))
  (bind _spline (`self.Spline`))
  (bind _returnvalue (`AddComponent|NODE_AddBoxComponent-1`))
  (bind _output_get (set `self.BeginBox` _returnvalue))
  (`SceneComponent.K2_SetRelativeLocation` (`self.BeginBox`) (`SplineComponent.GetLocationAtDistanceAlongSpline` (`self.Spline`) 0.0 "Local") false true)
  (`BoxComponent.SetBoxExtent` _output_get (32.0 32.0 32.0) true)
  (bind _returnvalue_2 (`AddComponent|NODE_AddBoxComponent-0`))
  (`SceneComponent.K2_SetRelativeLocation` _returnvalue_2 (`SplineComponent.GetLocationAndTangentAtSplinePoint` _spline (`SplineComponent.GetNumberOfSplinePoints` _spline) "Local") false true)
  (bind _output_get_2 (set `self.EndBox` _returnvalue_2))
  (`BoxComponent.SetBoxExtent` _output_get_2 (32.0 32.0 32.0) true))