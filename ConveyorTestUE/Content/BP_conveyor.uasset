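; BP_conveyor is a spline-driven conveyor actor that builds its shape from repeated spline mesh sections, with no active runtime logic.
; Its construction script scales SectionLength by the actor's Y scale, then adds one spline mesh per whole section along the spline, dropping any remainder.
; Each piece takes local spline positions and a start tangent clamped to section length, while the end tangent is clamped to zero.
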(fn `UserConstructionScript`
  (bind (_returnvalue_x _returnvalue_y) (`KismetMathLibrary.BreakVector` (`self.GetActorScale3D`)))
  (set `self.SectionLength` (* (`self.SectionLength`) _returnvalue_y))
  (for _index (range (`KismetMathLibrary.FTrunc` (/ (`SplineComponent.GetSplineLength` (`self.SplineComponent`)) (`self.SectionLength`))))
    (bind _returnvalue (`AddComponent|NODE_AddSplineMeshComponent-0`))
    (bind _returnvalue_2 (* _index (`self.SectionLength`)))
    (bind _returnvalue_3 (* (+ _index 1) (`self.SectionLength`)))
    (`SplineMeshComponent.SetStartAndEnd` _returnvalue (`SplineComponent.GetLocationAtDistanceAlongSpline` (`self.SplineComponent`) _returnvalue_2 "Local") (`KismetMathLibrary.ClampVectorSize` (`SplineComponent.GetTangentAtDistanceAlongSpline` (`self.SplineComponent`) _returnvalue_2 "Local") 0.0 (`self.SectionLength`)) (`SplineComponent.GetLocationAtDistanceAlongSpline` (`self.SplineComponent`) _returnvalue_3 "Local") (`KismetMathLibrary.ClampVectorSize` (`SplineComponent.GetTangentAtDistanceAlongSpline` (`self.SplineComponent`) _returnvalue_3 "Local")) true)))