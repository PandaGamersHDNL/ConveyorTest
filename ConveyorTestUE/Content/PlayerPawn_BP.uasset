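; Player pawn Blueprint that can be carried along a spline like a conveyor.
; SetMove stores the spline reference and turns movement on or off, without resetting the travelled distance.
; While movement is on, Tick does a swept move to the world location at the current spline distance, then advances that distance by ConveyorSpeed scaled by delta time.
; Only location is updated, not rotation.
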(event `self.ReceiveTick`
  (params (DeltaSeconds :type "Float (single-precision)"))
  (if (`self.ConveyorMove?`)
    (`self.K2_SetActorLocation` (`SplineComponent.GetLocationAtDistanceAlongSpline` (`self.SplineRefrence`) (`self.ConveyorDistance`) "World") true)
    (set `self.ConveyorDistance` (+ (* DeltaSeconds (`self.ConveyorSpeed`)) (`self.ConveyorDistance`)))))

(fn `SetMove`
  (params (`Conveyor Move` :type Boolean) (Spline :type "SplineComponent Object Reference"))
  (set `self.ConveyorMove?` `Conveyor Move`)
  (set `self.SplineRefrence` Spline))

(fn `UserConstructionScript`)