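; Spline conveyor for hoppers that carries Items between trigger boxes the construction script builds at each end of the spline.
; Items entering the begin box start moving along the spline, each linked to the previous one as its FrontItem.
; An OutPut overlapping that box becomes the conveyor's owner, and a spline point snaps to it.
; The end box stops Items and player pawns; the player's boarding logic is disconnected.
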(event `self.BeginBox.OnComponentBeginOverlap`
  (params (OverlappedComponent :type "PrimitiveComponent Object Reference") (OtherActor :type "Actor Object Reference") (OtherComp :type "PrimitiveComponent Object Reference") (OtherBodyIndex :type Integer) (bFromSweep :type Boolean) (SweepResult :type "HitResult Structure (by ref)"))
  (bind _asitem (cast `/Game/Item` OtherActor)
    (:`then`
      (`/Game/Item.Move Item?` _asitem true (`self.Spline`))
      (set `/Game/Item.FrontItem` (`self.LastItem`) _asitem)
      (set `/Game/Item.ConveyorDistance` 0.0 _asitem)
      (set `self.LastItem` _asitem))
    (:`CastFailed`
      (bind _asout_put (cast `/Game/OutPut` OtherActor))
      (`self.SetOwner` _asout_put)
      (`SplineComponent.SetLocationAtSplinePoint` (`self.Spline`) 0 (`self.K2_GetActorLocation` _asout_put) "World" true)
      (set `/Game/OutPut.ownedConveyor` self _asout_put)
      (`KismetSystemLibrary.PrintString` "Hello"))))

(event `self.EndBox.OnComponentBeginOverlap`
  (params (OverlappedComponent :type "PrimitiveComponent Object Reference") (OtherActor :type "Actor Object Reference") (OtherComp :type "PrimitiveComponent Object Reference") (OtherBodyIndex :type Integer) (bFromSweep :type Boolean) (SweepResult :type "HitResult Structure (by ref)"))
  (bind _spline (`self.Spline`))
  (bind _asplayer_pawn_bp (cast `/Game/PlayerPawn_BP` OtherActor)
    (:`then`
      (`/Game/PlayerPawn_BP.SetMove` _asplayer_pawn_bp false _spline))
    (:`CastFailed`
      (bind _asitem (cast `/Game/Item` OtherActor))
      (`/Game/Item.Move Item?` _asitem false _spline))))

(fn `UserConstructionScript`
  (locals (NewLocalVar_0 :type "BoxComponent Object Reference"))
  (bind _spline (`self.Spline`))
  (bind _returnvalue (`AddComponent|NODE_AddBoxComponent-1`))
  (bind _output_get (set `self.BeginBox` _returnvalue))
  (`SceneComponent.K2_SetRelativeLocation` (`self.BeginBox`) (`SplineComponent.GetLocationAtDistanceAlongSpline` (`self.Spline`) 0.0 "Local") false true)
  (`BoxComponent.SetBoxExtent` _output_get (32.0 32.0 32.0) true)
  (bind _returnvalue_2 (`AddComponent|NODE_AddBoxComponent-0`))
  (`SceneComponent.K2_SetRelativeLocation` _returnvalue_2 (`SplineComponent.GetLocationAndTangentAtSplinePoint` _spline (`SplineComponent.GetNumberOfSplinePoints` _spline) "Local") false true)
  (bind _output_get_2 (set `self.EndBox` _returnvalue_2))
  (`BoxComponent.SetBoxExtent` _output_get_2 (32.0 32.0 32.0) true))